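; Blueprint library of easing functions that reshape an input T along sine, bounce, quadratic and quintic curves.
; Each function is an independent single expression, with no state or shared helper.
; The two sine names are swapped relative to convention: EaseInShine decelerates and EaseOutShine accelerates.
; EaseInBounce is not normalized: its decaying bounces peak well above 1 and return to zero at T=1.
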(fn `easeInBounce`
  (params (t :type "Float (double-precision)"))
  (returns (res :type "Float (double-precision)"))
  (return (* (`KismetMathLibrary.Abs` (`KismetMathLibrary.Sin` (* (`KismetMathLibrary.MultiplyByPi` t) 3.5))) (`KismetMathLibrary.MultiplyMultiply_FloatFloat` (* (- t 1.0) 6.0) 2.0))))

(fn `easeInQuad`
  (params (ttt :type "Float (double-precision)"))
  (returns (res :type "Float (double-precision)"))
  (return (* ttt ttt)))

(fn `easeInQuint`
  (params (ttt :type "Float (double-precision)"))
  (returns (res :type "Float (double-precision)"))
  ;[1 1 1] t * t2 * t2
  (return (* ttt (* ttt ttt) (* ttt ttt))))

(fn `easeInShine`
  (params (t :type "Float (double-precision)"))
  (returns (res :type "Float (double-precision)"))
  (return (`KismetMathLibrary.Sin` (* t 1.570796))))

(fn `easeOutShine`
  (params (t :type "Float (double-precision)"))
  (returns (res :type "Float (double-precision)"))
  (return (+ (`KismetMathLibrary.Sin` (* (- t 1.0) 1.570796)) 1.0)))